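; BP_Agent is a steering-behavior agent that moves a physics Cone using Seek, currently aimed at the world origin.
; BeginPlay gives the Cone an initial velocity, then Tick calls Seek and applies the resulting CurrentVel as linear velocity.
; Seek subtracts the Cone's location plus velocity from the offset to target, then adds that normalized, force-scaled vector to velocity, without delta-time scaling.
; Optional debug arrows show current, desired and steering vectors.
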(event EventBeginPlay
  (bind _cone (Variables|Default|GetCone))
  (Physics|SetPhysicsLinearVelocity _cone "100.000000,100.000000,0.000000" false "None")
  (Variables|Default|SetCurrentVel (Transformation|GetComponentVelocity _cone)))

(event Collision|EventActorBeginOverlap
  (params (OtherActor :type Actor%20Object%20Reference)))

(event EventTick
  (params (DeltaSeconds :type Float%20%28single-precision%29))
  (CallFunction|Seek "0, 0, 0" true 1e+02)
  (Physics|SetPhysicsLinearVelocity (Variables|Default|GetCone) (Variables|Default|GetCurrentVel) false "None"))

(fn ConstructionScript)

(fn Seek
  (params (DesiredPos :type Vector) (Debug :type Boolean) (SteeringForce :type Float%20%28double-precision%29))
  (bind _cone (Variables|Default|GetCone))
  (bind _cone_2 (Variables|Default|GetCone))
  (bind _returnvalue (Transformation|GetWorldLocation _cone))
  (bind _returnvalue_2 (Transformation|GetWorldLocation _cone_2))
  (LocalVariables|Set_CurrentPos DesiredPos)
  (LocalVariables|Set_Debug Debug)
  (LocalVariables|SetSteeringMagnitude SteeringForce)
  (Utilities|FlowControl|Sequence
    (:then_0
      ;[0.15 0.15 0.15 0.5] Debug CV
      (if (LocalVariables|Get_Debug)
        (Rendering|Debug|DrawDebugArrow _returnvalue_2 (+ _returnvalue_2 (Variables|Default|GetCurrentVel)) 2e+01 "(R=0.074510,G=0.149020,B=0.082353,A=1.000000)" 0.0 1e+01)))
    (:then_1
      ;[0.1412 0.07451 0.149 0.502] Desired Vel Vector
      (LocalVariables|SetDesiredVel (- (LocalVariables|Get_CurrentPos) (Transformation|GetWorldLocation (Variables|Default|GetCone)))))
    (:then_2
      ;[0.15 0.15 0.15 0.5] Debug DV
      (if (LocalVariables|Get_Debug)
        (Rendering|Debug|DrawDebugArrow _returnvalue (+ _returnvalue (LocalVariables|GetDesiredVel)) 2e+01 "(R=0.141176,G=0.074510,B=0.149020,A=1.000000)" 0.0 1e+01)))
    (:then_3
      ;[0.149 0.03137 0.03137 0.502] Steering Vel
      (bind _output_get (LocalVariables|SetSteering (- (LocalVariables|GetDesiredVel) (+ (Transformation|GetWorldLocation (Variables|Default|GetCone)) (Transformation|GetComponentVelocity (Variables|Default|GetCone))))))
      ;[0.8549 0.3804 0.05098 0.502] Normalized Steering
      (bind _output_get_2 (LocalVariables|SetN_Steering (Math|Vector|Normalize _output_get)))
      (LocalVariables|SetFinalSteering (* _output_get_2 (LocalVariables|GetSteeringMagnitude))))
    (:then_4
      ;[0.15 0.15 0.15 0.5] Debug Steering
      (if (LocalVariables|Get_Debug)
        (Rendering|Debug|DrawDebugArrow (+ (Transformation|GetWorldLocation (Variables|Default|GetCone)) (Variables|Default|GetCurrentVel)) (+ (+ (Transformation|GetWorldLocation (Variables|Default|GetCone)) (Variables|Default|GetCurrentVel)) (LocalVariables|GetSteering)) 2e+01 "(R=0.149020,G=0.031373,B=0.031373,A=1.000000)" 0.0 1e+01)))
    (:then_5
      ;[0.15 0.15 0.15 0.5] Debug Final Steering
      (if (LocalVariables|Get_Debug)
        (Rendering|Debug|DrawDebugArrow (+ (Transformation|GetWorldLocation (Variables|Default|GetCone)) (Variables|Default|GetCurrentVel)) (+ (+ (Transformation|GetWorldLocation (Variables|Default|GetCone)) (Variables|Default|GetCurrentVel)) (LocalVariables|GetFinalSteering)) 2e+01 "(R=0.854902,G=0.380392,B=0.050980,A=1.000000)" 0.0 1e+01)))
    (:then_6
      ;[0.029 0.03324 0.2698 0.5] Desired Vel + Normalized Steering
      (Variables|Default|SetCurrentVel (+ (Transformation|GetComponentVelocity (Variables|Default|GetCone)) (LocalVariables|GetFinalSteering))))))